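; BP_ASV is a surface vessel actor, likely an ASV, that interacts with a fluid simulation and tracks its surge velocity.
; Shortly after BeginPlay it enables forces on Fluid, registers the hull as a dynamic force source, and hides itself from its scene capture.
; Each Tick differentiates world X/Y position and projects it onto yaw to get signed forward speed.
; An alternative force registration using a material override is left unconnected.
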(event `self.ReceiveBeginPlay`
  (bind _fluid (`self.Fluid`))
  (bind `_船体` (`self.船体`))
  (`KismetSystemLibrary.Delay` 0.1)
  (set `/Water/FluidSimulation/Blueprints/BP_FluidSim_01.Enabled` true _fluid)
  (set `/Water/FluidSimulation/Blueprints/BP_FluidSim_01.ApplyForces` 1.0 _fluid)
  (`/Water/FluidSimulation/Blueprints/BP_FluidSim_01.Register Dynamic Force` _fluid (make `/Water/FluidSimulation/Blueprints/Structs/FluidForceDynamic` "NewEnumerator0" 100.0 1.6 `_船体` "/Water/FluidSimulation/Materials/Forces/M_Fluid_Sim_Force_Boat_Component.M_Fluid_Sim_Force_Boat_Component") `_船体` 0.0)
  (`SceneCaptureComponent.HideActorComponents` (`self.SceneCaptureComponent2D`) self true))

(event `self.ReceiveTick`
  (params (DeltaSeconds :type "Float (single-precision)"))
  (bind _yaw (.yaw (`self.K2_GetActorRotation` self)))
  ; 注释
  (bind _output_get (set `self.Historical_X` (`self.Current_X`)))
  (bind _output_get_2 (set `self.Current_X` (.x (`self.K2_GetActorLocation` self))))
  (bind _output_get_3 (set `self.Historical_Y` (`self.Current_Y`)))
  (bind _output_get_4 (set `self.Current_Y` (.y (`self.K2_GetActorLocation` self))))
  (set `self.Surge_Velocity` (+ (* (`KismetMathLibrary.SafeDivide` (- _output_get_2 _output_get) DeltaSeconds) (`KismetMathLibrary.DegCos` _yaw)) (* (`KismetMathLibrary.SafeDivide` (- _output_get_4 _output_get_3) DeltaSeconds) (`KismetMathLibrary.DegSin` _yaw)))))

(fn `UserConstructionScript`)