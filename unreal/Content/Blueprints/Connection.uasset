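; Bridge actor linking the simulated ASV to an external Jetson as a TCP client, using ObjectDeliverer with terminator-framed JSON.
; A looping timer sends JPEG camera captures, ASV state and four target boats' ASV-relative position and velocity.
; Received commands either set thruster strengths or, as validated, sequence-checked kinematic setpoints, teleport the ASV by local deltas and yaw it toward movement.
; Tick makes a CameraActor follow the ASV along X.
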(event `断开连接`
  (params (ClientSocket :type "ObjectDelivererProtocol Object Reference"))
  ; 创建Object Deliverer管理器
  (set `self.bJetsonConnected` false)
  (`|ExecutionSequence`
    (:`then_0`
      (set `self.LeftThruster` 0.0))
    (:`then_1`
      (set `self.RightThruster` 0.0))
    (:`then_2`
      (`KismetSystemLibrary.PrintText` "Disconnected" true true (struct :`R` 1.0 :`A` 1.0)))))

(event `成功连接`
  (params (ClientSocket :type "ObjectDelivererProtocol Object Reference"))
  ; 创建Object Deliverer管理器
  (set `self.bJetsonConnected` true)
  (`|ExecutionSequence`
    (:`then_0`
      (set `self.LeftThruster` 0.0))
    (:`then_1`
      (set `self.RightThruster` 0.0))
    (:`then_2`
      (`KismetSystemLibrary.PrintText` "Connected" true true (struct :`G` 1.0 :`A` 1.0)))))

(event `self.ReceiveBeginPlay`
  (`|ExecutionSequence`
    (:`then_0`
      ; 创建Object Deliverer管理器
      (bind _output_get (set `self.ConnectionManager` (`ObjectDelivererManager.CreateObjectDelivererManager` true)))
      (add `ObjectDelivererManager.Connected` _output_get (delegate `成功连接`))
      (add `ObjectDelivererManager.Disconnected` _output_get (delegate `断开连接`)))
    (:`then_1`
      ; 创建Message Box
      (bind _output_get_2 (set `self.MessageBox` (`DeliveryBoxFactory.CreateObjectDeliveryBoxUsingJson` "/Game/Blueprints/Message_Receive.Message_Receive_C")))
      (add `ObjectDeliveryBoxUsingJson.Received` _output_get_2 (delegate `接收数据`))
      (`KismetSystemLibrary.PrintText` "Binded"))
    (:`then_2`
      ; 创建服务器
      (`ObjectDelivererManager.Start` (`self.ConnectionManager`) (`ProtocolFactory.CreateProtocolTcpIpClient` "192.168.137.100" 8080 true true) (`PacketRuleFactory.CreatePacketRuleTerminate` (`ODStringUtil.StringToBuffer` "__OD_END__")) (`self.MessageBox`)))
    (:`then_3`
      (`KismetSystemLibrary.K2_SetTimerDelegate` (delegate `Send State To Jetson`) 0.1 true))
    (:`then_4`
      (set `self.Guid` (`KismetGuidLibrary.Conv_GuidToString` (`KismetGuidLibrary.NewGuid`))))
    (:`then_5`
      (set `self.FrameIndex` 0))))

(event `self.ReceiveTick`
  (params (DeltaSeconds :type "Float (single-precision)"))
  (bind _returnvalue_x (`KismetMathLibrary.BreakVector` (`self.K2_GetActorLocation` (`self.ASV`))))
  (bind _returnvalue (`GameplayStatics.GetActorOfClass` "/Script/Engine.CameraActor"))
  (`self.K2_SetActorLocation` _returnvalue (`KismetMathLibrary.MakeVector` _returnvalue_x -9500.0 700.0) false false))

(event `接收数据`
  (params (ReceivedObject :type "Object Object Reference") (ReceivedJsonString :type String) (FromObject :type "ObjectDelivererProtocol Object Reference"))
  (bind _asv (`self.ASV`))
  (bind _asv_2 (`self.ASV`))
  (bind _rotation (.rotation (`self.GetTransform` (`self.ASV`))))
  ; 创建Message Box
  (bind _outjsonobject (`JsonBlueprintFunctionLibrary.FromString` ReceivedJsonString))
  (bind _outvalue (`|GetJsonField` _outjsonobject "Command_Type"))
  (if (`KismetStringLibrary.EqualEqual_StrStr` _outvalue "Kinematic_Setpoint")
    ; 安全检查
    (bind _outvalue_2 (`|GetJsonField` _outjsonobject "Valid"))
    (bind _output_get (set `self.bValid` _outvalue_2))
    (if _output_get
      (bind _outvalue_3 (`|GetJsonField` _outjsonobject "Hold_Position"))
      (bind _output_get_2 (set `self.bHoldPosition` _outvalue_3))
      (if (not _output_get_2)
        (bind _outvalue_4 (`|GetJsonField` _outjsonobject "Sequence"))
        (bind _output_get_3 (set `self.Sequence` _outvalue_4))
        (if (> _output_get_3 (`self.LastAppliedSequence`))
          (bind _outvalue_5 (`|GetJsonField` _outjsonobject "Delta_X_Cm"))
          (bind _output_get_4 (set `self.Delta_X_Cm` _outvalue_5))
          (bind _outvalue_6 (`|GetJsonField` _outjsonobject "Delta_Y_Cm"))
          (bind _output_get_5 (set `self.Delta_Y_Cm` _outvalue_6))
          (bind _returnvalue (`KismetMathLibrary.GreaterGreater_VectorRotator` (`KismetMathLibrary.MakeVector` _output_get_4 _output_get_5) _rotation))
          (`self.K2_SetActorLocation` _asv_2 (+ (.location (`self.GetTransform` (`self.ASV`))) _returnvalue) false true)
          (if (> (`KismetMathLibrary.VSize` _returnvalue) 0.0)
            (`self.K2_SetActorRotation` _asv_2 (`KismetMathLibrary.MakeRotator` (.roll _rotation) (.pitch _rotation) (.yaw (`KismetMathLibrary.MakeRotFromX` _returnvalue))) true)
            (set `self.LastAppliedSequence` (`self.Sequence`))))))
    (else
      (`|ExecutionSequence`
        (:`then_0`
          ; 控制ASV运动
          (bind _outvalue_7 (`|GetJsonField` _outjsonobject "Left_Thruster"))
          (bind _output_get_6 (set `self.LeftThruster` _outvalue_7)))
        (:`then_1`
          (bind _outvalue_8 (`|GetJsonField` _outjsonobject "Right_Thruster"))
          (bind _output_get_7 (set `self.RightThruster` _outvalue_8))
          (`|ExecutionSequence`
            (:`then_0`
              (set `PhysicsThrusterComponent.ThrustStrength` _output_get_6 (`/Game/BP_ASV.左推进器` _asv)))
            (:`then_1`
              (set `PhysicsThrusterComponent.ThrustStrength` _output_get_7 (`/Game/BP_ASV.右推进器` _asv)))))))))

(event `Send State To Jetson`
  (bind _asv (`self.ASV`))
  (bind _target (`self.Target`))
  (bind _asv_2 (`self.ASV`))
  (bind _json (`self.Json`))
  (bind _target1 (`self.Target1`))
  (bind _asv_3 (`self.ASV`))
  (bind _json1 (`self.Json1`))
  (bind _target2 (`self.Target2`))
  (bind _asv_4 (`self.ASV`))
  (bind _json2 (`self.Json2`))
  (bind _json3 (`self.Json3`))
  (bind _target3 (`self.Target3`))
  (bind _asv_5 (`self.ASV`))
  (bind _returnvalue (`self.GetTransform` _asv))
  (bind _returnvalue_2 (`self.GetTransform` _asv_2))
  (bind _returnvalue_3 (`self.GetTransform` _asv_3))
  (bind _returnvalue_4 (`self.GetTransform` _asv_4))
  (if (`self.bJetsonConnected`)
    ; 构建并发送消息
    (bind _outjpegdata (`ImageCompressionLibrary.CompressRenderTargetToJPEG` (`self.RenderResult`) 50))
    (`|SetJsonField` _json "RelativePosition" (`KismetMathLibrary.InverseTransformLocation` _returnvalue_2 (`self.K2_GetActorLocation` _target)))
    (`|SetJsonField` _json "RelativeVelocity" (`KismetMathLibrary.InverseTransformDirection` _returnvalue_2 (- (`self.GetVelocity` _target) (`self.GetVelocity` _asv_2))))
    (`|SetJsonField` _json "Entity_Id" "target_red")
    (`|SetJsonField` _json "Class" "boat")
    (`|SetJsonField` _json "Color" "red")
    (`|SetJsonField` _json "Is_Target" true)
    (`|SetJsonField` _json "Visible" true)
    (`|SetJsonField` _json1 "RelativePosition" (`KismetMathLibrary.InverseTransformLocation` _returnvalue_3 (`self.K2_GetActorLocation` _target1)))
    (`|SetJsonField` _json1 "RelativeVelocity" (`KismetMathLibrary.InverseTransformDirection` _returnvalue_3 (- (`self.GetVelocity` _target1) (`self.GetVelocity` _asv_3))))
    (`|SetJsonField` _json1 "Entity_Id" "target_blue")
    (`|SetJsonField` _json1 "Class" "boat")
    (`|SetJsonField` _json1 "Color" "blue")
    (`|SetJsonField` _json1 "Is_Target" true)
    (`|SetJsonField` _json1 "Visible" true)
    (`|SetJsonField` _json2 "RelativePosition" (`KismetMathLibrary.InverseTransformLocation` _returnvalue_4 (`self.K2_GetActorLocation` _target2)))
    (`|SetJsonField` _json2 "RelativeVelocity" (`KismetMathLibrary.InverseTransformDirection` _returnvalue_4 (- (`self.GetVelocity` _target2) (`self.GetVelocity` _asv_4))))
    (`|SetJsonField` _json2 "Entity_Id" "target_left")
    (`|SetJsonField` _json2 "Class" "boat")
    (`|SetJsonField` _json2 "Color" "white")
    (`|SetJsonField` _json2 "Is_Target" true)
    (`|SetJsonField` _json2 "Visible" true)
    (`|SetJsonField` _json3 "RelativePosition" (`KismetMathLibrary.InverseTransformLocation` _returnvalue (`self.K2_GetActorLocation` _target3)))
    (`|SetJsonField` _json3 "RelativeVelocity" (`KismetMathLibrary.InverseTransformDirection` _returnvalue (- (`self.GetVelocity` _target3) (`self.GetVelocity` _asv))))
    (`|SetJsonField` _json3 "Entity_Id" "target_right")
    (`|SetJsonField` _json3 "Class" "boat")
    (`|SetJsonField` _json3 "Color" "white")
    (`|SetJsonField` _json3 "Is_Target" true)
    (`|SetJsonField` _json3 "Visible" true)
    (bind _returnvalue_5 (`|GenericCreateObject` "/Game/Blueprints/Message_Send.Message_Send_C" (`KismetSystemLibrary.GetGameTimeInSeconds`) _outjpegdata (`/Game/BP_ASV.Surge_Velocity` _asv_5) (.z (`PrimitiveComponent.GetPhysicsAngularVelocityInDegrees` (`/Game/BP_ASV.船体` _asv_5) "None")) (`SceneComponent.K2_GetComponentLocation` (`/Game/BP_ASV.SceneCaptureComponent2D` _asv_5)) (`self.K2_GetActorRotation` _asv_5) (`SceneComponent.K2_GetComponentLocation` (`/Game/BP_Target.船体` (`self.Target`))) (`|MakeArray` _json _json1 _json2 _json3) (`self. SceneSeed`) (`self.Guid`) (`self.FrameIndex`)))
    (`ObjectDeliveryBoxUsingJson.Send` (`self.MessageBox`) _returnvalue_5)
    (`/Engine/EditorBlueprintResources/StandardMacros.IncrementInt` (`self.FrameIndex`))))

(fn `UserConstructionScript`)