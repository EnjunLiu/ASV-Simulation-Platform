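; BP_Target is a target boat actor whose hull (船体) interacts with a fluid simulation.
; Shortly after BeginPlay it registers the hull with Fluid as a dynamic force; Tick checks the Jetson connection but takes no action.
; Disconnected logic holds an alternate force registration and a timed weaving path, alternating straight runs with mirrored sine-derived turns that would drive hull velocity and actor yaw.
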(event `self.ReceiveTick`
  (params (DeltaSeconds :type "Float (single-precision)"))
  (if (`/Game/Blueprints/Connection.bJetsonConnected` (`self.ConnectionReference`))
    _))

(event `self.ReceiveBeginPlay`
  (bind `_船体` (`self.船体`))
  (`KismetSystemLibrary.Delay` 0.25)
  (`/Water/FluidSimulation/Blueprints/BP_FluidSim_01.Register Dynamic Force` (`self.Fluid`) (make `/Water/FluidSimulation/Blueprints/Structs/FluidForceDynamic` "NewEnumerator0" 100.0 1.4 `_船体` "/Water/FluidSimulation/Materials/Forces/M_Fluid_Sim_Force_Boat_Component.M_Fluid_Sim_Force_Boat_Component") `_船体` 0.0))

(fn `UserConstructionScript`)